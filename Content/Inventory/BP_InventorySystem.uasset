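; BP_InventorySystem is an inventory component with empty add and remove functions; its working logic detects the actor the player is looking at.
; Every tick it sphere-traces from the owner's location along the camera's forward vector, out to InteractionRange.
; On a hit it stores the actor as LookAtActor and prints its LookAtMessage.
; An extra Visibility line trace only draws a debug line, as its result is unused.
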(event EventTick
  (params (DeltaSeconds :type Float%20%28single-precision%29))
  (CallFunction|InteractionTrace))

(fn AddtoInventory)

(fn RemovefromInventory)

(fn InteractionTrace
  (bind _returnvalue (Game|GetPlayerCameraManager 0))
  (bind _returnvalue_2 (Components|GetOwner))
  (bind _interactionrange (Variables|Default|GetInteractionRange))
  (bind _returnvalue_3 (Transformation|GetActorLocation _returnvalue_2))
  (bind _returnvalue_4 (Transformation|GetActorForwardVector _returnvalue))
  (bind _returnvalue_5 (* _returnvalue_4 _interactionrange))
  (bind _returnvalue_6 (+ _returnvalue_3 _returnvalue_5))
  (bind (_outhit _returnvalue_7) (Collision|SphereTraceByChannel _returnvalue_3 _returnvalue_6 15.0 "TraceTypeQuery3" false (Utilities|Array|MakeArray _returnvalue_2) "None"))
  (if _returnvalue_7
    (Collision|LineTraceByChannel _returnvalue_3 _returnvalue_6 "TraceTypeQuery1" false 0 "ForDuration" true "(R=0.130209,G=0.039631,B=1.000000,A=1.000000)")
    (bind _output_get (Variables|Default|SetLookAtActor (.HitActor (Collision|BreakHitResult _outhit))))
    (bind _message (Class|IInteractInterface|Lookat(Message) _output_get))
    (Development|PrintString (Utilities|String|ToString(Text) _message))))